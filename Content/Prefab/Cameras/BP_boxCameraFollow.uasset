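; BP_boxCameraFollow is a trigger box that switches the player's view to a camera that turns to track the character.
; When BP_ThirdPersonCharacter overlaps the box, it sets the Camera as player 0's view target and starts LookAtPlayer.
; LookAtPlayer re-aims the camera through a self-calling short Delay loop gated by CanRotate, which this graph never clears.
; The construction script sizes the box from InBoxExtent.
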(event `self.Box.OnComponentBeginOverlap`
  (params (OverlappedComponent :type "PrimitiveComponent Object Reference") (OtherActor :type "Actor Object Reference") (OtherComp :type "PrimitiveComponent Object Reference") (OtherBodyIndex :type Integer) (bFromSweep :type Boolean) (SweepResult :type "HitResult Structure (by ref)"))
  (bind _asbp_third_person_character (cast `/Game/ThirdPerson/Blueprints/BP_ThirdPersonCharacter` OtherActor))
  (`PlayerController.SetViewTargetWithBlend` (`GameplayStatics.GetPlayerController` 0) (`self.Camera`) 0.0 "VTBlend_Linear" 0.0 false)
  (set `self.CanRotate` true)
  (`self.LookAtPlayer`))

(event `LookAtPlayer`
  (bind _camera (`self.Camera`))
  (if (`self.CanRotate`)
    (`self.K2_SetActorRotation` _camera (`KismetMathLibrary.FindLookAtRotation` (`self.K2_GetActorLocation` _camera) (`self.K2_GetActorLocation` (stale `self.Box.OnComponentBeginOverlap` _asbp_third_person_character))) false)
    (`KismetSystemLibrary.Delay` 0.005)
    (`self.LookAtPlayer`)))

(fn `UserConstructionScript`
  (`BoxComponent.SetBoxExtent` (`self.Box`) (`self.In Box Extent`) true))